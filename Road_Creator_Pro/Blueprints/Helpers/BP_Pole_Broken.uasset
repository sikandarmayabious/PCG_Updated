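; Broken roadside pole actor that plays an impact sound when it appears and later removes itself.
; On BeginPlay it maps CarSpeed, converted to km/h, to the hit sound's volume and pitch, with slight random variation.
; Tick destroys the actor once the player camera is over 100 meters away, or after a 20-second delay if no valid camera manager exists.
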(event `self.ReceiveBeginPlay`
  (bind _returnvalue (* (`self.Car Speed`) 0.036))
  (`GameplayStatics.PlaySoundAtLocation` "/Game/Road_Creator_Pro/Sound/S_Pole_Hit.S_Pole_Hit" (`self.K2_GetActorLocation`) (struct) (+ (`KismetMathLibrary.MapRangeClamped` _returnvalue 3.0 80.0 0.2 0.8) (`KismetMathLibrary.RandomFloatInRange` -0.1 0.1)) (+ (`KismetMathLibrary.MapRangeClamped` _returnvalue 3.0 80.0 0.35 0.8) (`KismetMathLibrary.RandomFloatInRange` -0.1 0.1)) 0.0 null null null null))

(event `self.ReceiveTick`
  (params (DeltaSeconds :type "Float (single-precision)"))
  (bind _returnvalue (`GameplayStatics.GetPlayerCameraManager` 0))
  ;[1 1 1] Actor Self-Destroy
  (if (`KismetSystemLibrary.IsValid` _returnvalue)
    (if (> (`KismetMathLibrary.Vector_Distance` (`PlayerCameraManager.GetCameraLocation` _returnvalue) (`self.K2_GetActorLocation`)) 10000.0)
      (`self.K2_DestroyActor` :!label _label))
    (else
      (`KismetSystemLibrary.Delay` 20.0)
      (goto _label))))

(fn `UserConstructionScript`)